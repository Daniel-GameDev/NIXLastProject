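; BP_CourseActor is a lesson actor that switches between a couch and a chair as other actors enter and leave its box.
; BeginPlay binds the box overlap events, which pass the overlapping actor and new mesh to ChangeMesh and set the 3D widget's text to match.
; Every tick, the widget turns on yaw only to face the player pawn, using a look-at rotation from the mesh's location.
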(event `self.ReceiveBeginPlay`
  (bind _boxcollision (`self.BoxCollision`))
  (add `PrimitiveComponent.OnComponentBeginOverlap` _boxcollision (delegate `OnComponentBeginOverlap_Box`))
  (add `PrimitiveComponent.OnComponentEndOverlap` _boxcollision (delegate `OnComponentEndOverlap_Event_0`)))

(event `OnComponentBeginOverlap_Box`
  (params (OverlappedComponent :type "PrimitiveComponent Object Reference") (OtherActor :type "Actor Object Reference") (OtherComp :type "PrimitiveComponent Object Reference") (OtherBodyIndex :type Integer) (bFromSweep :type Boolean) (SweepResult :type "HitResult Structure (by ref)"))
  (`self.ChangeMesh` OtherActor "/Game/StarterContent/Props/SM_Couch.SM_Couch")
  (bind _asumg_3dwidget (cast `/Game/Course/Lesson7/UMG_3DWidget` (`WidgetComponent.GetWidget` (`self.WidgetComponent`))))
  (`TextBlock.SetText` (`/Game/Course/Lesson7/UMG_3DWidget.Text` _asumg_3dwidget) "Couch"))

(event `OnComponentEndOverlap_Event_0`
  (params (OverlappedComponent :type "PrimitiveComponent Object Reference") (OtherActor :type "Actor Object Reference") (OtherComp :type "PrimitiveComponent Object Reference") (OtherBodyIndex :type Integer))
  (`self.ChangeMesh` OtherActor "/Game/StarterContent/Props/SM_Chair.SM_Chair")
  (bind _asumg_3dwidget (cast `/Game/Course/Lesson7/UMG_3DWidget` (`WidgetComponent.GetWidget` (`self.WidgetComponent`))))
  (`TextBlock.SetText` (`/Game/Course/Lesson7/UMG_3DWidget.Text` _asumg_3dwidget) "Chair"))

(event `self.ReceiveTick`
  (params (DeltaSeconds :type "Float (single-precision)"))
  (`SceneComponent.K2_SetWorldRotation` (`self.WidgetComponent`) (`KismetMathLibrary.MakeRotator` 0.0 0.0 (.yaw (`KismetMathLibrary.FindLookAtRotation` (`SceneComponent.K2_GetComponentLocation` (`self.Mesh`)) (`self.K2_GetActorLocation` (`GameplayStatics.GetPlayerPawn` 0))))) false false))

(fn `UserConstructionScript`)