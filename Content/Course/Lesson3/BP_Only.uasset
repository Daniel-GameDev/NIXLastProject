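; BP_Only is a lesson Blueprint that swaps its static mesh when the player pawn enters or leaves a trigger box.
; On BeginPlay it binds handlers to the Box component's begin and end overlap events.
; Overlap by player 0's pawn shows the couch mesh, and leaving switches it to the chair mesh.
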(event `self.ReceiveBeginPlay`
  (bind _box (`self.Box`))
  (add `PrimitiveComponent.OnComponentBeginOverlap` _box (delegate `OnComponentBeginOverlap_Box`))
  (add `PrimitiveComponent.OnComponentEndOverlap` _box (delegate `OnComponentEndOverlap_Box`)))

(event `OnComponentBeginOverlap_Box`
  (params (OverlappedComponent :type "PrimitiveComponent Object Reference") (OtherActor :type "Actor Object Reference") (OtherComp :type "PrimitiveComponent Object Reference") (OtherBodyIndex :type Integer) (bFromSweep :type Boolean) (SweepResult :type "HitResult Structure (by ref)"))
  (if (== OtherActor (`GameplayStatics.GetPlayerPawn` 0))
    (`StaticMeshComponent.SetStaticMesh` (`self.StaticMesh`) "/Game/StarterContent/Props/SM_Couch.SM_Couch")))

(event `OnComponentEndOverlap_Box`
  (params (OverlappedComponent :type "PrimitiveComponent Object Reference") (OtherActor :type "Actor Object Reference") (OtherComp :type "PrimitiveComponent Object Reference") (OtherBodyIndex :type Integer))
  (if (== OtherActor (`GameplayStatics.GetPlayerPawn` 0))
    (`StaticMeshComponent.SetStaticMesh` (`self.StaticMesh`) "/Game/StarterContent/Props/SM_Chair.SM_Chair")))

(fn `UserConstructionScript`)